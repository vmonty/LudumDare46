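; Water-style projectile that irrigates and damages whatever it hits, and destroys itself on impact or after a set lifetime.
; A hit sends the Irrigable discrete message to the other actor, applies damage and spawns a splash effect at the impact point.
; The construction script gives the mesh a dynamic material with a randomized RandomMesh parameter for visual variation.
; An attached splash effect at the player's fire point is present but disconnected.
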(event EventBeginPlay
  (Utilities|FlowControl|Delay (Variables|Default|GetTimeToDestroy))
  (Actor|DestroyActor))

(event Collision|EventHit
  (params (MyComp :type Primitive%20Component%20Object%20Reference) (Other :type Actor%20Object%20Reference) (OtherComp :type Primitive%20Component%20Object%20Reference) (bSelfMoved :type Boolean) (HitLocation :type Vector :default "0, 0, 0") (HitNormal :type Vector :default "0, 0, 0") (NormalImpulse :type Vector :default "0, 0, 0") (Hit :type Hit%20Result%20Structure%20%28by%20ref%29))
  (Class|BPIIrrigable|IrrigableDiscrete(Message) Other)
  (Game|Damage|ApplyDamage Other (Variables|Default|GetBaseDamage) 0 0)
  (Effects|SpawnEmitteratLocation "/Game/VFX/PS_Splash_Impact.PS_Splash_Impact" HitLocation)
  (Actor|DestroyActor))

(fn ConstructionScript
  (bind _returnvalue (Rendering|Material|CreateDynamicMaterialInstance "/Game/VFX/Material/M_Proyectile.M_Proyectile" "None" :!class /Script/Engine.KismetMaterialLibrary))
  (Rendering|Material|SetMaterial (Variables|Default|GetProjectileMesh) 0 _returnvalue)
  (Rendering|Material|SetScalarParameterValue _returnvalue "RandomMesh" (Math|Conversions|ToFloat(Integer) (Math|Random|RandomInteger 2)) :!class /Script/Engine.MaterialInstanceDynamic))