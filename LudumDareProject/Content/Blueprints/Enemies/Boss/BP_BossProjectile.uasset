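; Boss projectile actor that damages what it hits and spawns a BP_EnemyTomato_Mini enemy at the impact point.
; On hit it plays a sound, sends the hit actor an irrigation message, applies damage and shows a splash effect before destroying itself.
; Without a hit it destroys itself after TimeToDestroy.
; An unconnected branch that would attach a splash emitter to the player's fire point never runs.
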(event EventBeginPlay
  (Utilities|FlowControl|Delay (Variables|Default|GetTimeToDestroy))
  (Actor|DestroyActor))

(event Collision|EventHit
  (params (MyComp :type Primitive%20Component%20Object%20Reference) (Other :type Actor%20Object%20Reference) (OtherComp :type Primitive%20Component%20Object%20Reference) (bSelfMoved :type Boolean) (HitLocation :type Vector :default "0, 0, 0") (HitNormal :type Vector :default "0, 0, 0") (NormalImpulse :type Vector :default "0, 0, 0") (Hit :type Hit%20Result%20Structure%20%28by%20ref%29))
  (Audio|PlaySoundatLocation "/Game/Sounds/Effects/ShotHit_Cue.ShotHit_Cue" HitLocation "0, 0, 0" 1.0 1.0 0.0 0 0 0)
  (Class|BPIIrrigable|IrrigableDiscrete(Message) Other)
  (Game|Damage|ApplyDamage Other (Variables|Default|GetBaseDamage) 0 0)
  (Effects|SpawnEmitteratLocation "/Game/VFX/PS_Splash_Impact.PS_Splash_Impact" HitLocation)
  (Game|SpawnActorfromClass "/Game/Blueprints/Enemies/Boss/BP_EnemyTomato_Mini.BP_EnemyTomato_Mini_C" (Math|Transform|MakeTransform HitLocation "0, 0, 0" "1,1,1") "AlwaysSpawn" 0 0)
  (Actor|DestroyActor))

(fn ConstructionScript)