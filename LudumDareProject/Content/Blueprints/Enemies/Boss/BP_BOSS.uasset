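; Tomato monster boss that, once BossSpawn fires, shows a health bar, plays random voice lines and fights the player.
; A Tick-driven state machine faces the player and cycles idle, hop and projectile shot, with AttackArea overlap triggering a damaging melee hit.
; Damage feeds BPHealthComponent and the bar; death plays slow-motion, swaps to the dead mesh, awards money and shows the WIN screen.
; An unconnected old-enemy death branch remains.
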(event OnComponentBeginOverlap(AttackArea)
  (params (OverlappedComponent :type Primitive%20Component%20Object%20Reference) (OtherActor :type Actor%20Object%20Reference) (OtherComp :type Primitive%20Component%20Object%20Reference) (OtherBodyIndex :type Integer) (bFromSweep :type Boolean) (SweepResult :type Hit%20Result%20Structure%20%28by%20ref%29))
  ;[0 0 0] State Machine
  ;;[1 1 1] AttackTrigger
  (if (== OtherActor (Game|GetPlayerCharacter 0))
    (Variables|Default|SetState "NewEnumerator2")))

(event Custom|BossSpawn
  (bind _returnvalue (Transformation|GetActorLocation))
  (bind _bp_health_component (Variables|Default|GetBP_Health_Component))
  ;[1 1 1] Begin
  (Variables|Default|SetBossSpawned true)
  (bind _returnvalue_2 (UserInterface|CreateWidget "/Game/Blueprints/UI/W_BossHealth.W_BossHealth_C" (Game|GetPlayerController 0)))
  (Variables|Default|SetBoss%20UI _returnvalue_2)
  (Variables|/Game/Blueprints/UI/W_BossHealth.W_BossHealth_C|SetBossHealth _returnvalue_2 (/ (Variables|/Game/Blueprints/Components/BP_Health_Component.BP_Health_Component_C|GetCurrentHealth _bp_health_component) (Variables|/Game/Blueprints/Components/BP_Health_Component.BP_Health_Component_C|GetMaxHealth _bp_health_component)))
  (UserInterface|Viewport|AddtoViewport _returnvalue_2 0)
  (Utilities|FlowControl|Delay (Math|Random|RandomFloatinRange 2.0 8.0) :!label _label)
  (if (Math|Random|RandomBool)
    (Audio|PlaySoundatLocation "/Game/Sounds/Effects/TomatoVoice1_Cue.TomatoVoice1_Cue" _returnvalue "0, 0, 0" 1.0 1.0 0.0 0 0 0)
    (goto _label)
    (else
      (Audio|PlaySoundatLocation "/Game/Sounds/Effects/TomatoVoice2_Cue.TomatoVoice2_Cue" _returnvalue "0, 0, 0" 1.0 1.0 0.0 0 0 0)
      (goto _label))))

(event EventBeginPlay)

(event Game|Damage|EventAnyDamage
  (params (Damage :type Float%20%28single-precision%29) (DamageType :type Damage%20Type%20Object%20Reference) (InstigatedBy :type Controller%20Object%20Reference) (DamageCauser :type Actor%20Object%20Reference))
  (bind _bp_health_component (Variables|Default|GetBP_Health_Component))
  ;[1 1 1] Damage
  (Audio|PlaySoundatLocation "/Game/Sounds/Effects/EnemyHit_Cue.EnemyHit_Cue" (Transformation|GetActorLocation) "0, 0, 0" 1.0 1.0 0.0 0 0 0)
  (Default|TakeDamage (Variables|Default|GetBP_Health_Component) Damage)
  (Variables|/Game/Blueprints/UI/W_BossHealth.W_BossHealth_C|SetBossHealth (Variables|Default|GetBoss%20UI) (/ (Variables|/Game/Blueprints/Components/BP_Health_Component.BP_Health_Component_C|GetCurrentHealth _bp_health_component) (Variables|/Game/Blueprints/Components/BP_Health_Component.BP_Health_Component_C|GetMaxHealth _bp_health_component)))
  (if (<= (Variables|/Game/Blueprints/Components/BP_Health_Component.BP_Health_Component_C|GetCurrentHealth (Variables|Default|GetBP_Health_Component)) 0.0)
    ;;[1 0.4531 0.4531] Dead
    (Utilities|FlowControl|DoOnce false
      (:Completed
        (Default|FadeOutUI (Variables|Default|GetBoss%20UI))
        (Rendering|SetVisibility (Variables|Character|GetMesh) false true)
        (Rendering|SetVisibility (Variables|Default|GetBossDead) true false)
        (Components|Animation|PlayAnimation (Variables|Default|GetBossDead) "/Game/Characters/Boss/BossDead_Anim.BossDead_Anim" false)
        ;;;[1 1 1] Slowmo
        (Utilities|FlowControl|Delay 0.2)
        (Utilities|Time|SetGlobalTimeDilation 0.35)
        (Utilities|FlowControl|Delay 3.0)
        (Utilities|Time|SetGlobalTimeDilation 1.0)
        (Collision|SetCollisionEnabled (Variables|Collision|GetCapsuleComponent) "NoCollision")
        (Utilities|FlowControl|Sequence
          (:then_0
            ;;[1 1 1] Loot money
            (Effects|SpawnEmitteratLocation "/Game/VFX/Plants/PS_BossCoins.PS_BossCoins" (Transformation|GetActorLocation))
            (Audio|PlaySound2D "/Game/Sounds/Effects/GetMoney.GetMoney" 1.0 1.0 0.0 0 0)
            (bind _asbp_player_character (Utilities|Casting|CastToBP_PlayerCharacter (Game|GetPlayerCharacter 0)))
            (Default|IncrementMoney _asbp_player_character))
          (:then_1
            ;;[0.5359 0.659 1] Win UI
            (Utilities|FlowControl|Delay 6.0)
            (bind _asbp_player_character_2 (Utilities|Casting|CastToBP_PlayerCharacter (Game|GetPlayerCharacter 0)))
            (Class|BPGameJamKitHUDInterface|ShowGameOver(Message) (HUD|GetHUD (Game|GetPlayerController 0)) "WIN" (Utilities|Text|ToText(Integer) (Variables|/Game/Blueprints/Player/BP_PlayerCharacter.BP_PlayerCharacter_C|GetMoney _asbp_player_character_2)))
            (Actor|DestroyActor)))))))

(event EventTick
  (params (DeltaSeconds :type Float%20%28single-precision%29))
  (bind _returnvalue (Game|GetPlayerCharacter 0))
  (bind _returnvalue_2 (Transformation|GetActorLocation))
  (bind _returnvalue_3 (Transformation|GetActorForwardVector))
  (bind _returnvalue_4 (Transformation|GetActorForwardVector))
  (bind _shootpoint (Variables|Default|GetShootPoint))
  (bind _returnvalue_5 (Transformation|GetActorLocation _returnvalue))
  (bind _returnvalue_6 (* _returnvalue_3 -1e+02))
  (bind _returnvalue_7 (* _returnvalue_4 6e+02))
  (bind _returnvalue_8 (Transformation|GetWorldLocation _shootpoint))
  (bind _returnvalue_9 (Math|Rotator|FindLookatRotation _returnvalue_2 _returnvalue_5))
  ;[0 0 0] State Machine
  (if (and (Variables|Default|GetBossSpawned) (>= (Variables|/Game/Blueprints/Components/BP_Health_Component.BP_Health_Component_C|GetCurrentHealth (Variables|Default|GetBP_Health_Component)) 0.1))
    (Transformation|SetActorRotation (Math|Rotator|MakeRotator (.roll _returnvalue_9) 0.0 (.yaw _returnvalue_9)))
    (switch Utilities|FlowControl|Switch|SwitchonEEnemyTomatoBossState (Variables|Default|GetState)
      (:NewEnumerator0
        ;;[1 0.9577 0.4914] Idle
        (if (AI|Components|NavMovement|IsFalling (Variables|Character|GetCharacterMovement))
          (Variables|Default|SetCanPush true)
          (if (Variables|Default|GetCanHop)
            (Components|Animation|PlayAnimation (Variables|Character|GetMesh) "/Game/Characters/A_TomatoMonster_Jump_Anim.A_TomatoMonster_Jump_Anim" true)
            (Variables|Default|SetCanHop false))
          (else
            (Variables|Default|SetCanHop true)
            (if (Variables|Default|GetCanPush)
              (Components|Animation|PlayAnimation (Variables|Character|GetMesh) "/Game/Characters/A_TomatoMonster_Push.A_TomatoMonster_Push" false)
              (Variables|Default|SetCanPush false))
            (Utilities|FlowControl|Delay 1.0)
            (if (Utilities|Enum|Equal(Enum) (Variables|Default|GetState) "NewEnumerator0")
              (Variables|Default|SetState "NewEnumerator1")))))
      (:NewEnumerator1
        ;;[0.5785 1 0.7191] Hop
        (Character|LaunchCharacter (Math|Vector|MakeVector (.x _returnvalue_7) (.y _returnvalue_7) 6e+02) true true)
        (if (>= (Math|Random|RandomInteger 10) 4)
          (Variables|Default|SetState "NewEnumerator0")
          (else
            (Variables|Default|SetState "NewEnumerator3"))))
      (:NewEnumerator2
        ;;[1 0.3698 0.3698] Attack
        (bind _asbp_player_character (Utilities|Casting|CastToBP_PlayerCharacter (Game|GetPlayerCharacter 0)))
        (Game|Damage|ApplyDamage _asbp_player_character (Variables|Default|GetAttackDamage) 0 0)
        (Character|LaunchCharacter (Math|Vector|MakeVector (.x _returnvalue_6) (.y _returnvalue_6) -2.5e+02) true true)
        (Variables|Default|SetState "NewEnumerator0"))
      (:NewEnumerator3
        ;;[0.5077 0.9502 1] Shoot
        (Game|SpawnActorfromClass "/Game/Blueprints/Enemies/Boss/BP_BossProjectile.BP_BossProjectile_C" (Math|Transform|MakeTransform _returnvalue_8 (Math|Rotator|FindLookatRotation _returnvalue_8 (Transformation|GetActorLocation (Game|GetPlayerCharacter 0))) "1,1,1") "Undefined" 0 0)
        (Variables|Default|SetState "NewEnumerator0")))))

(fn ConstructionScript)