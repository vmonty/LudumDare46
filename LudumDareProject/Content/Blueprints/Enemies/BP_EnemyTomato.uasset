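; Tomato enemy that hops toward the player, deals damage on contact and can drop a healing pickup on death.
; A Tick-driven state switch turns it toward the player and uses LaunchCharacter to hop forward after a grounded idle delay.
; Overlapping the attack area triggers damage and a backward recoil launch.
; Incoming damage goes to a health component; at zero it spawns a particle effect, rolls for the pickup and destroys itself.
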(event OnComponentBeginOverlap(AttackArea)
  (params (OverlappedComponent :type Primitive%20Component%20Object%20Reference) (OtherActor :type Actor%20Object%20Reference) (OtherComp :type Primitive%20Component%20Object%20Reference) (OtherBodyIndex :type Integer) (bFromSweep :type Boolean) (SweepResult :type Hit%20Result%20Structure%20%28by%20ref%29))
  (if (== OtherActor (Game|GetPlayerCharacter 0))
    (Variables|Default|SetState "NewEnumerator2")))

(event Game|Damage|EventAnyDamage
  (params (Damage :type Float%20%28single-precision%29) (DamageType :type Damage%20Type%20Object%20Reference) (InstigatedBy :type Controller%20Object%20Reference) (DamageCauser :type Actor%20Object%20Reference))
  (bind _returnvalue (Transformation|GetActorLocation))
  (bind (_x _y) (Math|Vector|BreakVector _returnvalue))
  (bind _returnvalue_2 (Math|Vector|MakeVector _x _y 4e+01))
  (Default|TakeDamage (Variables|Default|GetBP_Health_Component) Damage)
  (if (<= (Variables|/Game/Blueprints/Components/BP_Health_Component.BP_Health_Component_C|GetCurrentHealth (Variables|Default|GetBP_Health_Component)) 0.0)
    (Effects|SpawnEmitteratLocation "/Game/VFX/Enemies/PS_DieTomato.PS_DieTomato" _returnvalue)
    (bind _output_get (Variables|Default|SetChoosenNumber (Math|Random|RandomInteger (Variables|Default|GetTotalOfNumbersToChoose))))
    (if (== _output_get (Variables|Default|GetCorrectNumberToHeal))
      (Game|SpawnActorfromClass "/Game/Blueprints/EnviromentProps/BP_HealingPickUp.BP_HealingPickUp_C" (Math|Transform|MakeTransform _returnvalue_2 "0, 0, 0" "1,1,1") "AdjustIfPossibleButAlwaysSpawn" 0 0)
      ;[1 0.01361 0] SOUND - TODO
      (Audio|PlaySoundatLocation 0 _returnvalue_2 "0, 0, 0" 1.0 1.0 0.0 0 0 0)
      (Actor|DestroyActor)
      (else
        (Actor|DestroyActor)))))

(event EventTick
  (params (DeltaSeconds :type Float%20%28single-precision%29))
  (bind _returnvalue (Game|GetPlayerCharacter 0))
  (bind _returnvalue_2 (Transformation|GetActorLocation))
  (bind _returnvalue_3 (Transformation|GetActorForwardVector))
  (bind _returnvalue_4 (Transformation|GetActorForwardVector))
  (bind _returnvalue_5 (Transformation|GetActorLocation _returnvalue))
  (bind _returnvalue_6 (* _returnvalue_3 -3e+02))
  (bind _returnvalue_7 (* _returnvalue_4 3e+02))
  (bind _returnvalue_8 (Math|Rotator|FindLookatRotation _returnvalue_2 _returnvalue_5))
  (Transformation|SetActorRotation (Math|Rotator|MakeRotator (.roll _returnvalue_8) 0.0 (.yaw _returnvalue_8)))
  (switch Utilities|FlowControl|Switch|SwitchonEEnemyTomatoState (Variables|Default|GetState)
    (:NewEnumerator0
      (Utilities|FlowControl|Delay 1.2)
      (if (Utilities|Enum|Equal(Enum) (Variables|Default|GetState) "NewEnumerator0")
        (if (not (AI|Components|NavMovement|IsFalling (Variables|Character|GetCharacterMovement)))
          (Variables|Default|SetState "NewEnumerator1"))))
    (:NewEnumerator1
      (Character|LaunchCharacter (Math|Vector|MakeVector (.x _returnvalue_7) (.y _returnvalue_7) 3.5e+02) true true)
      (Variables|Default|SetState "NewEnumerator0"))
    (:NewEnumerator2
      (bind _asbp_player_character (Utilities|Casting|CastToBP_PlayerCharacter (Game|GetPlayerCharacter 0)))
      (Game|Damage|ApplyDamage _asbp_player_character (Variables|Default|GetAttackDamage) 0 0)
      (Character|LaunchCharacter (Math|Vector|MakeVector (.x _returnvalue_6) (.y _returnvalue_6) 3.5e+02) true true)
      (Variables|Default|SetState "NewEnumerator0"))))

(fn ConstructionScript)