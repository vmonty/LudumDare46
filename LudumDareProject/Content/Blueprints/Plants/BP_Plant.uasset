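; BP_Plant is a plant actor with a water level that governs whether it progresses toward its next growth state or toward death.
; Tick raises water while watered (Space, for debug), otherwise drains it after a delay, running the evolve timer while wet and the death timer when dry.
; UpdateUI feeds all three values to progress-bar widgets.
; LaunchState events swap materials; nothing here calls them or acts on expired timers.
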(event Custom|LaunchState3
  (if (not (>= (Variables|Default|GetCurrentState) 3))
    (Rendering|Material|SetMaterial (Variables|Default|GetPlant) 0 "/Game/Materials/M_PlantState3.M_PlantState3")
    (Variables|Default|SetCurrentState (+ (Variables|Default|GetCurrentState) 1))))

(event Custom|LaunchState2
  (if (not (>= (Variables|Default|GetCurrentState) 2))
    (Rendering|Material|SetMaterial (Variables|Default|GetPlant) 0 "/Game/Materials/M_PlantState2.M_PlantState2")
    (Variables|Default|SetCurrentState (+ (Variables|Default|GetCurrentState) 1))))

(event EventBeginPlay
  ;[1 1 1] DEBUG
  (Input|EnableInput (Game|GetPlayerController 0))
  (Rendering|Material|SetMaterial (Variables|Default|GetPlant) 0 "/Game/Materials/M_PlantState1.M_PlantState1")
  (Variables|Default|SetCurrentState (+ (Variables|Default|GetCurrentState) 1))
  (Variables|Default|SetCurrentWaterLevel (Variables|Default|GetInitialWaterLevel))
  (Variables|Default|SetCurrentTimeToDie (Utilities|Array|Get(acopy) (Variables|Default|GetTimeToDie)))
  (Variables|Default|SetCurrentTimeToNextState (Utilities|Array|Get(acopy) (Variables|Default|GetTimeToNextState)))
  (CallFunction|UpdateUI))

(event Collision|EventActorBeginOverlap
  (params (OtherActor :type Actor%20Object%20Reference)))

(event EventTick
  (params (DeltaSeconds :type Float%20%28single-precision%29))
  (Development|PrintString (Utilities|String|Append "CurrentTimeToDie: " (Utilities|String|ToString(Float) (Variables|Default|GetCurrentTimeToDie)) " 
CurrentTimeToNextState: " (Utilities|String|ToString(Float) (Variables|Default|GetCurrentTimeToNextState))) true true "(R=0.000000,G=0.660000,B=1.000000,A=1.000000)" 1.0)
  (Variables|Default|SetTempDeltaSeconds DeltaSeconds)
  (Utilities|FlowControl|Sequence
    (:then_0
      (if (Variables|Default|GetIsBeingWatered)
        (Variables|Default|SetCurrentWaterLevel (Math|Float|Clamp(Float) (+ (Variables|Default|GetCurrentWaterLevel) (* (Variables|Default|GetTempDeltaSeconds) (Variables|Default|GetWaterLevelDecreaseSpeed))) 0.0 (Variables|Default|GetMaxWaterLevel)))
        (elif (> (Variables|Default|GetCurrentWaterDecrementDelay) 0.0)
          (Variables|Default|SetCurrentWaterDecrementDelay (- (Variables|Default|GetCurrentWaterDecrementDelay) (Variables|Default|GetTempDeltaSeconds)))
          (else
            (Variables|Default|SetCurrentWaterLevel (Math|Float|Clamp(Float) (- (Variables|Default|GetCurrentWaterLevel) (* (Variables|Default|GetTempDeltaSeconds) (Variables|Default|GetWaterLevelDecreaseSpeed))) 0.0 (Variables|Default|GetMaxWaterLevel)))))))
    (:then_1
      (if (> (Variables|Default|GetCurrentWaterLevel) 0.0)
        (Variables|Default|SetCurrentTimeToNextState (- (Variables|Default|GetCurrentTimeToNextState) (Variables|Default|GetTempDeltaSeconds)))
        (else
          (Variables|Default|SetCurrentTimeToDie (- (Variables|Default|GetCurrentTimeToDie) (Variables|Default|GetTempDeltaSeconds))))))
    (:then_2
      (CallFunction|UpdateUI))))

(event Input|KeyboardEvents|SpaceBar
  (params (Key :type Key%20Structure :default "None"))
  ;[1 1 1] DEBUG
  (:Pressed
    (Variables|Default|SetIsBeingWatered true))
  (:Released
    (Variables|Default|SetIsBeingWatered false)
    (Variables|Default|SetCurrentWaterDecrementDelay (Variables|Default|GetWaterDecrementDelay))))

(fn ConstructionScript)

(fn UpdateUI
  (bind _aswater_level_ui (Utilities|Casting|CastToWaterLevel_UI (UserInterface|GetUserWidgetObject (Variables|Default|GetWaterLevelProgressBar))))
  (Default|SetPercent _aswater_level_ui (/ (Variables|Default|GetCurrentWaterLevel) (Variables|Default|GetMaxWaterLevel)))
  ;[1 1 1] DEBUG
  (bind _aswater_level_ui_2 (Utilities|Casting|CastToWaterLevel_UI (UserInterface|GetUserWidgetObject (Variables|Default|GetTimeToEvolveProgressBar))))
  (Default|SetPercent _aswater_level_ui_2 (/ (Variables|Default|GetCurrentTimeToNextState) (Utilities|Array|Get(acopy) (Variables|Default|GetTimeToNextState))))
  (bind _aswater_level_ui_3 (Utilities|Casting|CastToWaterLevel_UI (UserInterface|GetUserWidgetObject (Variables|Default|GetTimeToDieProgressBar))))
  (Default|SetPercent _aswater_level_ui_3 (/ (Variables|Default|GetCurrentTimeToDie) (Utilities|Array|Get(acopy) (Variables|Default|GetTimeToDie)))))