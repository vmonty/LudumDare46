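; BP_HealingPickUp is an environment pickup that restores health to the player character on overlap.
; A timeline started on BeginPlay drives the cube mesh's relative Z position to animate it.
; Sphere overlap with BP_PlayerCharacter passes HealAmount once to its health component's ModifyHealth, spawns a particle effect and destroys the pickup after a brief delay.
; The pickup sound call is a TODO with no sound assigned.
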(event OnComponentBeginOverlap(Sphere)
  (params (OverlappedComponent :type Primitive%20Component%20Object%20Reference) (OtherActor :type Actor%20Object%20Reference) (OtherComp :type Primitive%20Component%20Object%20Reference) (OtherBodyIndex :type Integer) (bFromSweep :type Boolean) (SweepResult :type Hit%20Result%20Structure%20%28by%20ref%29))
  (bind _asbp_player_character (Utilities|Casting|CastToBP_PlayerCharacter OtherActor))
  (Utilities|FlowControl|DoOnce false
    (:Completed
      (Default|ModifyHealth (Variables|/Game/Blueprints/Player/BP_PlayerCharacter.BP_PlayerCharacter_C|GetBP_Health_Component _asbp_player_character) (Variables|Default|GetHeal%20Amount))
      (Effects|SpawnEmitteratLocation "/Game/VFX/Enviro/PS_HealthPicked.PS_HealthPicked" (Transformation|GetActorLocation))
      ;[1 0.0141 0] Sound - TODO
      (Audio|PlaySoundatLocation 0 (Transformation|GetWorldLocation (Variables|Default|GetDefaultSceneRoot)) "0, 0, 0" 1.0 1.0 0.0 0 0 0)
      (Utilities|FlowControl|Delay 0.1)
      (Actor|DestroyActor))))

(event EventBeginPlay
  (bind _newtrack_0 (Timeline|Timeline_0 Play)
    (:Update
      (Transformation|SetRelativeLocation (Variables|Default|GetCube) (Math|Vector|MakeVector 0.0 0.0 (* _newtrack_0 1e+01)) false false))))

(event Collision|EventActorBeginOverlap
  (params (OtherActor :type Actor%20Object%20Reference)))

(event EventTick
  (params (DeltaSeconds :type Float%20%28single-precision%29)))

(fn ConstructionScript)