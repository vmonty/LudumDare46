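; Environment prop that refills the player character's water can while the player stands inside its sphere collision.
; Overlap events toggle an in-range flag and spawn a recharge particle effect, which is destroyed after a short delay on exit.
; While in range, Tick adds water scaled by delta time and prints the can's level on screen.
; An alternative timer-driven interval recharge remains in the graph but is disconnected.
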(event OnComponentBeginOverlap(SphereCollision)
  (params (OverlappedComponent :type Primitive%20Component%20Object%20Reference) (OtherActor :type Actor%20Object%20Reference) (OtherComp :type Primitive%20Component%20Object%20Reference) (OtherBodyIndex :type Integer) (bFromSweep :type Boolean) (SweepResult :type Hit%20Result%20Structure%20%28by%20ref%29))
  (bind _returnvalue (Transformation|GetActorLocation))
  ;[1 1 1] Continuous amount
  (if (== OtherActor (Variables|Default|GetPlayerCharacter))
    (Variables|Default|SetIsPlayerOnRange true)
    ;;[1 0 0.03281] VFX del prop al recargar agua - TODO
    (bind _returnvalue_2 (Effects|SpawnEmitteratLocation "/Game/VFX/Player/PS_WaterRecharge.PS_WaterRecharge" (Math|Vector|MakeVector (.x _returnvalue) (.y _returnvalue) (+ (.z _returnvalue) 5.0)) "0, 0, 0" "1.000000,1.000000,1.000000" false))))

(event OnComponentEndOverlap(SphereCollision)
  (params (OverlappedComponent :type Primitive%20Component%20Object%20Reference) (OtherActor :type Actor%20Object%20Reference) (OtherComp :type Primitive%20Component%20Object%20Reference) (OtherBodyIndex :type Integer))
  ;[1 1 1] Continuous amount
  (if (== OtherActor (Variables|Default|GetPlayerCharacter))
    (Variables|Default|SetIsPlayerOnRange false)
    (Utilities|FlowControl|Delay 1.2)
    (Components|DestroyComponent (stale OnComponentBeginOverlap(SphereCollision) _returnvalue_2))))

(event Custom|RechargeActivated
  ;[1 1 1] Discrete amount
  (if (Variables|Default|GetIsPlayerOnRange)
    (Default|ModifyWaterLevel (Variables|Default|GetPlayerCharacter) (* (Variables|Default|GetQuantityOfWaterPerInterval) (Utilities|Time|GetWorldDeltaSeconds)))))

(event EventBeginPlay
  ;[0.9951 0.3077 1] Initial Setup
  (bind _asbp_player_character (Utilities|Casting|CastToBP_PlayerCharacter (Game|GetPlayerCharacter 0)))
  (Variables|Default|SetPlayerCharacter _asbp_player_character))

(event EventTick
  (params (DeltaSeconds :type Float%20%28single-precision%29))
  ;[1 1 1] Continuous amount
  (if (Variables|Default|GetIsPlayerOnRange)
    (Development|PrintString (Utilities|String|ToString(Float) (Variables|/Game/Blueprints/Player/BP_PlayerCharacter.BP_PlayerCharacter_C|GetWaterCanLevel (Variables|Default|GetPlayerCharacter))) true false "(R=0.000000,G=0.660000,B=1.000000,A=1.000000)" (Utilities|Time|GetWorldDeltaSeconds))
    (Default|ModifyWaterLevel (Variables|Default|GetPlayerCharacter) (* (Variables|Default|GetQuantityOfWaterPerInterval) (Utilities|Time|GetWorldDeltaSeconds)))))

(fn ConstructionScript)