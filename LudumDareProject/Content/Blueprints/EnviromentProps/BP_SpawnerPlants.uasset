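; Environment spawner that scatters actors of a configurable plant class at random horizontal offsets around itself, up to a maximum count.
; StartSpawning waits an initial delay, activates the spawner, spawns the first plant and starts a looping one-second countdown timer.
; While active, Tick spawns another plant when the countdown runs out, resets the interval and prints a debug string.
; Spawns avoid collisions, and only successful ones count toward the cap.
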(event Custom|Start%20Spawning
  (bind _defaultsceneroot (Variables|Default|GetDefaultSceneRoot))
  (bind _returnvalue (Transformation|GetWorldLocation _defaultsceneroot))
  (Utilities|FlowControl|Delay (Variables|Default|GetInitialDelay))
  (Variables|Default|SetIsActive true)
  (bind _returnvalue_2 (Game|SpawnActorfromClass (Variables|Default|GetClassOfPlant) (Math|Transform|MakeTransform (Math|Vector|MakeVector (+ (.x _returnvalue) (Math|Random|RandomFloatinRange -3.5e+02 3.5e+02)) (+ (.y _returnvalue) (Math|Random|RandomFloatinRange -3.5e+02 3.5e+02)) (.z _returnvalue)) "0, 0, 0" "1,1,1") "AdjustIfPossibleButDontSpawnIfColliding" 0 0))
  (Utilities|Time|SetTimerbyEvent (delegate Custom|Decrease%20A%20Second) 1.0 true)
  ;[1 1 1] Comment
  (Utilities|IsValid _returnvalue_2
    (:Is%20Valid
      (Variables|Default|SetActorsSpawned (+ (Variables|Default|GetActorsSpawned) 1)))))

(event Custom|Decrease%20A%20Second
  (Variables|Default|SetCurrentIntervalToSpawn (- (Variables|Default|GetCurrentIntervalToSpawn) 1.0))
  (if (>= (Variables|Default|GetCurrentIntervalToSpawn) (Variables|Default|GetIntervalToSpawn))
    _))

(event EventBeginPlay)

(event Collision|EventActorBeginOverlap
  (params (OtherActor :type Actor%20Object%20Reference)))

(event EventTick
  (params (DeltaSeconds :type Float%20%28single-precision%29))
  (bind _defaultsceneroot (Variables|Default|GetDefaultSceneRoot))
  (bind _returnvalue (Transformation|GetWorldLocation _defaultsceneroot))
  (if (Variables|Default|GetIsActive)
    (if (<= (Variables|Default|GetCurrentIntervalToSpawn) 0.0)
      (if (< (Variables|Default|GetActorsSpawned) (Variables|Default|GetMaxActorsToSpawn))
        (Development|PrintString (Utilities|String|Append "Current interval" (Utilities|String|ToString(Float) (Variables|Default|GetCurrentIntervalToSpawn))))
        (bind _returnvalue_2 (Game|SpawnActorfromClass (Variables|Default|GetClassOfPlant) (Math|Transform|MakeTransform (Math|Vector|MakeVector (+ (.x _returnvalue) (Math|Random|RandomFloatinRange -3.5e+02 3.5e+02)) (+ (.y _returnvalue) (Math|Random|RandomFloatinRange -3.5e+02 3.5e+02)) (.z _returnvalue)) "0, 0, 0" "1,1,1") "AdjustIfPossibleButDontSpawnIfColliding" 0 0))
        (Variables|Default|SetCurrentIntervalToSpawn (Variables|Default|GetIntervalToSpawn))
        (Utilities|IsValid _returnvalue_2
          (:Is%20Valid
            (Variables|Default|SetActorsSpawned (+ (Variables|Default|GetActorsSpawned) 1))))))))

(fn ConstructionScript
  (Variables|Default|SetCurrentIntervalToSpawn (Variables|Default|GetIntervalToSpawn)))