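; BP_WaterRecharger_Small is an environment prop that refills the player's water while they stand inside its collision sphere.
; Sphere overlaps toggle an in-range flag, and Tick adds water scaled by delta time while it is set.
; Entering plays a recharge sound through a DoOnce-guarded audio component, destroyed on exit; BeginPlay spawns a persistent particle effect.
; The timer-driven discrete recharge and overlap-spawned effects are left disconnected.
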(event OnComponentBeginOverlap(SphereCollision)
  (params (OverlappedComponent :type Primitive%20Component%20Object%20Reference) (OtherActor :type Actor%20Object%20Reference) (OtherComp :type Primitive%20Component%20Object%20Reference) (OtherBodyIndex :type Integer) (bFromSweep :type Boolean) (SweepResult :type Hit%20Result%20Structure%20%28by%20ref%29))
  ;[1 1 1] Continuous amount
  (if (== OtherActor (Variables|Default|GetPlayerCharacter))
    (Utilities|FlowControl|Sequence
      (:then_0
        (Variables|Default|SetIsPlayerOnRange true))
      (:then_1
        (Utilities|FlowControl|DoOnce false
          (:Completed
            (bind _returnvalue (AddComponent|AddAudioComponent false))
            (bind _output_get (Variables|Default|SetAudioComponentReference _returnvalue))
            (Audio|Components|Audio|SetSound _output_get "/Game/Sounds/Effects/WaterRechargeCue.WaterRechargeCue")
            (Audio|Components|Audio|Play _output_get 0.0)))))))

(event OnComponentEndOverlap(SphereCollision)
  (params (OverlappedComponent :type Primitive%20Component%20Object%20Reference) (OtherActor :type Actor%20Object%20Reference) (OtherComp :type Primitive%20Component%20Object%20Reference) (OtherBodyIndex :type Integer))
  ;[1 1 1] Continuous amount
  (if (== OtherActor (Variables|Default|GetPlayerCharacter))
    (Variables|Default|SetIsPlayerOnRange false)
    (Utilities|IsValid (Variables|Default|GetAudioComponentReference)
      (:Is%20Valid
        (Components|DestroyComponent (Variables|Default|GetAudioComponentReference))
        (Utilities|FlowControl|DoOnce false) ; enters at Reset
      ))))

(event Custom|RechargeActivated
  ;[1 1 1] Discrete amount
  (if (Variables|Default|GetIsPlayerOnRange)
    (Default|ModifyWaterLevel (Variables|Default|GetPlayerCharacter) (* (Variables|Default|GetQuantityOfWaterPerInterval) (Utilities|Time|GetWorldDeltaSeconds)))))

(event EventBeginPlay
  (bind _returnvalue (Transformation|GetActorLocation))
  ;[0.9951 0.3077 1] Initial Setup
  (bind _asbp_player_character (Utilities|Casting|CastToBP_PlayerCharacter (Game|GetPlayerCharacter 0)))
  (Variables|Default|SetPlayerCharacter _asbp_player_character)
  (Effects|SpawnEmitteratLocation "/Game/VFX/Player/PS_WaterRecharge_Small.PS_WaterRecharge_Small" (Math|Vector|MakeVector (.x _returnvalue) (.y _returnvalue) (+ (.z _returnvalue) 5.0)) "0, 0, 0" "0.500000,0.500000,0.500000" false))

(event EventTick
  (params (DeltaSeconds :type Float%20%28single-precision%29))
  ;[1 1 1] Continuous amount
  (if (Variables|Default|GetIsPlayerOnRange)
    (Default|ModifyWaterLevel (Variables|Default|GetPlayerCharacter) (* (Variables|Default|GetQuantityOfWaterPerInterval) (Utilities|Time|GetWorldDeltaSeconds)))))

(fn ConstructionScript)