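; BP_Fence is an environment prop that builds a row of fence segments in its construction script, sized by an EndPoint vector.
; When EndPoint has horizontal extent, its full length divided by FenceDistance sets the count of added static mesh components.
; Each is attached to the Fence component and offset at regular spacing along negative local Y; EndPoint's direction is not used here.
; The event graph is empty.
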(event EventBeginPlay)

(event Collision|EventActorBeginOverlap
  (params (OtherActor :type Actor%20Object%20Reference)))

(event EventTick
  (params (DeltaSeconds :type Float%20%28single-precision%29)))

(fn ConstructionScript
  (if (Math|Vector|NotEqual(Vector) (* (Variables|Default|GetEndPoint) "1.000000,1.000000, 0") "0, 0, 0" 0.0001)
    (for _index (range 1 (Math|Float|Floor (/ (Math|Vector|VectorLength (Variables|Default|GetEndPoint)) (Variables|Default|GetFenceDistance))))
      (Variables|Default|SetLastIndex _index)
      (Components|StaticMesh|SetStaticMesh (Variables|Default|GetFence) "/Game/Meshes/fence.fence")
      (bind _returnvalue (AddComponent|AddStaticMeshComponent true))
      (Transformation|AttachComponentToComponent _returnvalue (Variables|Default|GetFence) "None" "KeepWorld" "KeepWorld" "KeepRelative" true)
      (Transformation|SetRelativeLocationAndRotation _returnvalue (Math|Vector|MakeVector 0.0 (* (Variables|Default|GetLastIndex) (* (Variables|Default|GetFenceDistance) -1.0)) 0.0) "0, 0, 0" false false))))