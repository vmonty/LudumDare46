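; BP_Plant is a plant actor that changes the material on its Plant component as it advances through growth or visual states.
; BeginPlay applies the state 1 material and increments CurrentState.
; The LaunchState2 and LaunchState3 custom events, not called within this Blueprint, each set a material and increment CurrentState unless it has reached their state number.
; LaunchState3 applies the same M_PlantState2 material as LaunchState2.
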(event Custom|LaunchState3
  (if (not (>= (Variables|Default|GetCurrentState) 3))
    (Rendering|Material|SetMaterial (Variables|Default|GetPlant) 0 "/Game/Materials/M_PlantState2.M_PlantState2")
    (Variables|Default|SetCurrentState (+ (Variables|Default|GetCurrentState) 1))))

(event Custom|LaunchState2
  (if (not (>= (Variables|Default|GetCurrentState) 2))
    (Rendering|Material|SetMaterial (Variables|Default|GetPlant) 0 "/Game/Materials/M_PlantState2.M_PlantState2")
    (Variables|Default|SetCurrentState (+ (Variables|Default|GetCurrentState) 1))))

(event EventBeginPlay
  (Rendering|Material|SetMaterial (Variables|Default|GetPlant) 0 "/Game/Materials/M_PlantState1.M_PlantState1")
  (Variables|Default|SetCurrentState (+ (Variables|Default|GetCurrentState) 1)))

(event Collision|EventActorBeginOverlap
  (params (OtherActor :type Actor%20Object%20Reference)))

(event EventTick
  (params (DeltaSeconds :type Float%20%28single-precision%29)))

(fn ConstructionScript)