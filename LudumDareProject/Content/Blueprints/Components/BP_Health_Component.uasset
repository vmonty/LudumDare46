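; Health component that tracks an actor's current health against a maximum, starting at full on BeginPlay.
; TakeDamage and HealAmount events change CurrentHealth directly without clamping, and both subtract their input, so HealAmount lowers health as written.
; A separate ModifyHealth function adds a signed amount and clamps the result between zero and MaxHealth, but neither event calls it.
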(event Custom|TakeDamage
  (params (Damage :type Float%20%28single-precision%29))
  (Variables|Default|SetCurrentHealth (- (Variables|Default|GetCurrentHealth) Damage)))

(event Custom|HealAmount
  (params (HealAmount :type Float%20%28single-precision%29))
  (Variables|Default|SetCurrentHealth (- (Variables|Default|GetCurrentHealth) HealAmount)))

(event EventBeginPlay
  (Variables|Default|SetCurrentHealth (Variables|Default|GetMaxHealth)))

(fn ModifyHealth
  (params (Amount :type Float%20%28single-precision%29))
  (if (>= (+ Amount (Variables|Default|GetCurrentHealth)) (Variables|Default|GetMaxHealth))
    (Variables|Default|SetCurrentHealth (Variables|Default|GetMaxHealth))
    (elif (<= (+ Amount (Variables|Default|GetCurrentHealth)) 0.0)
      (Variables|Default|SetCurrentHealth 0.0)
      (else
        (Variables|Default|SetCurrentHealth (+ Amount (Variables|Default|GetCurrentHealth)))))))