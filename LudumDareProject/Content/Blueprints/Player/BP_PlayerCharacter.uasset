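; Player character Blueprint for a robot with wheel and flower child actors, handling damage, death, water can level and money.
; Damage reduces the health component with camera shake and sound, then either swaps body, wheel and flower materials during a Delay-based invulnerability window or disables input before calling the controller's Kill.
; Helper functions clamp and check water and increment money.
; A legacy timer-based cooldown remains disconnected.
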(event Custom|CooldownSubstraction
  ;[1 1 1] Delay implementation - Legacy
)

(event EventBeginPlay
  (bind _asbp_player_controller (Utilities|Casting|CastToBP_PlayerController (Game|GetPlayerController 0)))
  (Variables|Default|SetPlayerController _asbp_player_controller))

(event Game|Damage|EventAnyDamage
  (params (Damage :type Float%20%28single-precision%29) (DamageType :type Damage%20Type%20Object%20Reference) (InstigatedBy :type Controller%20Object%20Reference) (DamageCauser :type Actor%20Object%20Reference))
  (bind _playercontroller (Variables|Default|GetPlayerController))
  (bind _playermesh (Variables|Default|GetPlayerMesh))
  (bind _returnvalue (Rendering|Material|GetMaterials _playermesh))
  ;[0.7333 0.3767 0] Damaged
  (if (Variables|Default|GetCanBeDamaged)
    (Default|ModifyHealth (Variables|Default|GetBP_Health_Component) (* Damage -1.0))
    (Variables|Default|SetCanBeDamaged false)
    (Camera|PlayWorldCameraShake "/Game/Blueprints/BP_CameraShake.BP_CameraShake_C" (Transformation|GetActorLocation) 1e+03 1e+03)
    ;;[1 0 0] SOUND
    (Audio|PlaySoundatLocation "/Game/Sounds/Effects/RobotDamaged_Cue.RobotDamaged_Cue" (Transformation|GetActorLocation self) "0, 0, 0" 1.0 1.0 0.0 0 0 0)
    ;;[1 1 1] Death Sequence
    (if (== (Variables|/Game/Blueprints/Components/BP_Health_Component.BP_Health_Component_C|GetCurrentHealth (Variables|Default|GetBP_Health_Component)) 0.0)
      ;;;[1 0 0] SOUND - TODO
      (Audio|PlaySound2D "/Game/Sounds/Effects/RobotDeath_Cue.RobotDeath_Cue" 1.0 1.0 0.0 0 0)
      (Input|DisableInput (Variables|Default|GetPlayerController))
      (Utilities|FlowControl|Delay (Variables|Default|GetTimeToKill))
      (Input|EnableInput _playercontroller)
      (Default|Kill _playercontroller)
      (else
        ;;[0.06496 1 0] Body and flower colors
        (Variables|Colors|SetBodyMaterials _returnvalue)
        (for _index (range 0 (- (Utilities|Array|Length _returnvalue) 1))
          (Rendering|Material|SetMaterial (Variables|Default|GetPlayerMesh) _index (Variables|Colors|GetDamageMat)))
        (bind _asbp_player_wheel (Utilities|Casting|CastToBP_PlayerWheel (Variables|/Script/Engine.ChildActorComponent|GetChildActor (Variables|Default|GetBP_PlayerWheel))))
        (Variables|Colors|SetWheelMaterials (Rendering|Material|GetMaterials (Variables|/Game/Blueprints/Player/BP_PlayerWheel.BP_PlayerWheel_C|GetWheel _asbp_player_wheel)))
        (for _index_2 (range 0 (- (Utilities|Array|Length (Rendering|Material|GetMaterials (Variables|/Game/Blueprints/Player/BP_PlayerWheel.BP_PlayerWheel_C|GetWheel _asbp_player_wheel))) 1))
          (Rendering|Material|SetMaterial (Variables|/Game/Blueprints/Player/BP_PlayerWheel.BP_PlayerWheel_C|GetWheel _asbp_player_wheel) _index_2 (Variables|Colors|GetDamageMat)))
        (bind _asbp_flower_power (Utilities|Casting|CastToBP_FlowerPower (Variables|/Script/Engine.ChildActorComponent|GetChildActor (Variables|Default|GetBP_FlowerPower))))
        (Variables|Colors|SetFlowerMaterial (Rendering|Material|GetMaterial (Variables|/Game/Blueprints/Player/BP_FlowerPower.BP_FlowerPower_C|GetSM_FlowerPower _asbp_flower_power) 1))
        (Rendering|Material|SetMaterial (Variables|/Game/Blueprints/Player/BP_FlowerPower.BP_FlowerPower_C|GetSM_FlowerPower _asbp_flower_power) 1 (Variables|Colors|GetFlowerDamageMat))
        (Utilities|FlowControl|Delay (Variables|Default|GetInvulnerabilityTime))
        ;;[0.06496 1 0] Restore body and flower colors
        (for _index_3 (range 0 (- (Utilities|Array|Length (Variables|Colors|GetBodyMaterials)) 1))
          (Rendering|Material|SetMaterial (Variables|Default|GetPlayerMesh) _index_3 (Utilities|Array|Get(acopy) (Variables|Colors|GetBodyMaterials) _index_3)))
        (bind _asbp_player_wheel_2 (Utilities|Casting|CastToBP_PlayerWheel (Variables|/Script/Engine.ChildActorComponent|GetChildActor (Variables|Default|GetBP_PlayerWheel))))
        (for _index_4 (range 0 (- (Utilities|Array|Length (Variables|Colors|GetWheelMaterials)) 1))
          (Rendering|Material|SetMaterial (Variables|/Game/Blueprints/Player/BP_PlayerWheel.BP_PlayerWheel_C|GetWheel _asbp_player_wheel_2) _index_4 (Utilities|Array|Get(acopy) (Variables|Colors|GetWheelMaterials) _index_4)))
        (bind _asbp_flower_power_2 (Utilities|Casting|CastToBP_FlowerPower (Variables|/Script/Engine.ChildActorComponent|GetChildActor (Variables|Default|GetBP_FlowerPower))))
        (Rendering|Material|SetMaterial (Variables|/Game/Blueprints/Player/BP_FlowerPower.BP_FlowerPower_C|GetSM_FlowerPower _asbp_flower_power_2) 1 (Variables|Colors|GetFlowerMaterial))
        (Variables|Default|SetCanBeDamaged true)))))

(fn ConstructionScript)

(fn ModifyWaterLevel
  (params (Quantity :type Float%20%28single-precision%29))
  (if (>= (+ Quantity (Variables|Default|GetWaterCanLevel)) (Variables|Default|GetMaxWaterCanLevel))
    (Variables|Default|SetWaterCanLevel (Variables|Default|GetMaxWaterCanLevel))
    (elif (<= (+ Quantity (Variables|Default|GetWaterCanLevel)) 0.0)
      (Variables|Default|SetWaterCanLevel 0.0)
      (else
        (Variables|Default|SetWaterCanLevel (+ Quantity (Variables|Default|GetWaterCanLevel)))))))

(fn HasEnoughWater
  (params (Amount :type Float%20%28single-precision%29))
  (return (>= (+ Amount (Variables|Default|GetWaterCanLevel)) 0.0)))

(fn IncrementMoney
  (Variables|Default|SetMoney (+ (Variables|Default|GetMoney) (Variables|Default|GetMoneyIncrement))))