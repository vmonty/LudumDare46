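; Player controller for a top-down twin-stick character with a water can, handling world-axis movement, aiming, irrigation, shooting, melee picking and a cursor widget.
; Each tick it aims by the last input device, using thumbstick angle or the mouse ray's intersection with a plane at the pawn.
; Irrigation and projectiles consume pawn water; irrigation slows movement and, like melee, messages sphere-traced actors.
; Dash teleports along movement input, stopping at traced hits, with a cooldown.
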(event EventTick
  (params (DeltaSeconds :type Float%20%28single-precision%29))
  ;[0.7333 0.3767 0] Aiming
  (Aim|UpdatePlayerAim)
  ;[1 0.019 0] todelete
  (Development|PrintString (Utilities|String|ToString(Float) (Variables|/Game/Blueprints/Player/BP_PlayerCharacter.BP_PlayerCharacter_C|GetWaterCanLevel (Variables|Default|GetPlayerPawn))) true false "(R=0.064963,G=1.000000,B=0.000000,A=1.000000)" (Utilities|Time|GetWorldDeltaSeconds)))

(event EventBeginPlay
  ;[0.9951 0.3077 1] Initial Setup
  (bind _asbp_player_character (Utilities|Casting|CastToBP_PlayerCharacter (Pawn|GetControlledPawn)))
  (Variables|Default|SetPlayerPawn _asbp_player_character)
  ;[0.9951 0.3077 1] UI
  (bind _returnvalue (UserInterface|CreateWidget "/Game/Blueprints/UI/BP_CursorImage.BP_CursorImage_C" self))
  (bind _output_get (Variables|Default|SetCursor%20Widget%20Reference _returnvalue))
  (UserInterface|Viewport|AddtoViewport _output_get 0))

(event Input|ActionEvents|InputActionFire
  (params (Key :type Key%20Structure :default "None"))
  (bind _playerpawn (Variables|Default|GetPlayerPawn))
  (bind _firepoint (Variables|/Game/Blueprints/Player/BP_PlayerCharacter.BP_PlayerCharacter_C|GetFirePoint _playerpawn))
  ;[0.7333 0.3767 0] Shoot
  (:Pressed
    (bind _haswater (Default|HasEnoughWater (Variables|Default|GetPlayerPawn) (* (Variables|Default|GetSubtractedWaterAmount) -1.0)))
    (if _haswater
      (Game|SpawnActorfromClass "/Game/Blueprints/BP_Projectile.BP_Projectile_C" (Math|Transform|MakeTransform (Transformation|GetWorldLocation _firepoint) (Transformation|GetWorldRotation _firepoint) "1,1,1") "AlwaysSpawn" 0 0)
      (Effects|SpawnEmitterAttached "/Game/VFX/PS_Splash.PS_Splash" (Variables|/Game/Blueprints/Player/BP_PlayerCharacter.BP_PlayerCharacter_C|GetPlayerMesh (Variables|Default|GetPlayerPawn)) "ShootPoint")
      (Irrigation|SubtractWater false))))

(event Input|ActionEvents|InputActionMelee
  (params (Key :type Key%20Structure :default "None"))
  ;[0.7333 0.3767 0] Melee
  (:Pressed
    (bind (_isobjectmatch _hitactor) (Irrigation|ObjectDetection (Variables|Irrigation|GetDetectionRange)))
    (if _isobjectmatch
      (Class|BPIPickable|Pick(Message) _hitactor))))

(event Input|ActionEvents|InputActionDash
  (params (Key :type Key%20Structure :default "None"))
  ;[0.7333 0.3767 0] Dash
  (:Pressed
    (if (> (Math|Vector|VectorLength (Transformation|GetVelocity (Variables|Default|GetPlayerPawn))) 0.0)
      (if (Variables|Dash|GetDashAllowed)
        (bind (_outhit _returnvalue) (Collision|SphereTraceForObjects (Transformation|GetActorLocation (Variables|Default|GetPlayerPawn)) (Dash|CalculateDashDestination) 1e+01 (Utilities|Array|MakeArray "ObjectTypeQuery1" "ObjectTypeQuery2") false (Utilities|Array|MakeArray self (Pawn|GetControlledPawn)) "None" true "(R=1.000000,G=0.000000,B=0.932746,A=1.000000)" "(R=1.000000,G=0.856711,B=0.000000,A=1.000000)"))
        (if _returnvalue
          (Variables|Default|SetDestLocation (.ImpactPoint (Collision|BreakHitResult _outhit)))
          (else
            (Variables|Default|SetDestLocation (Dash|CalculateDashDestination))))
        (Transformation|Teleport (Variables|Default|GetPlayerPawn) (Variables|Default|GetDestLocation) "0, 0, 0")
        (Variables|Dash|SetDashAllowed false)
        (Utilities|FlowControl|Delay (Variables|Dash|GetDashCooldown))
        (Variables|Dash|SetDashAllowed true)))))

(event Input|AxisEvents|InputAxisMoveForward
  (params (AxisValue :type Float%20%28single-precision%29))
  ;[0.7333 0.3767 0] Basic Movement
  (Pawn|Input|AddMovementInput (Variables|Default|GetPlayerPawn) "1.000000, 0, 0" (* AxisValue (Variables|Irrigation|GetIrrigationSlow)) false))

(event Input|AxisEvents|InputAxisMoveRight
  (params (AxisValue :type Float%20%28single-precision%29))
  ;[0.7333 0.3767 0] Basic Movement
  (Pawn|Input|AddMovementInput (Variables|Default|GetPlayerPawn) "0,1.000000, 0" (* AxisValue (Variables|Irrigation|GetIrrigationSlow)) false))

(event Input|AxisEvents|InputAxisIrrigate
  (params (AxisValue :type Float%20%28single-precision%29))
  ;[0.7333 0.3767 0] Irrigation
  (if (> AxisValue 0.5)
    (bind _haswater (Default|HasEnoughWater (Variables|Default|GetPlayerPawn) (* (Variables|Default|GetSubtractedWaterAmount) -1.0 (Utilities|Time|GetWorldDeltaSeconds))))
    (if _haswater
      (Variables|Irrigation|SetIrrigationSlow 0.5)
      (Irrigation|SubtractWater true)
      ;;[0.06496 1 0] FX Watering
      (Effects|SpawnEmitterAttached "/Game/VFX/Player/PS_Irriagation.PS_Irriagation" (Variables|/Game/Blueprints/Player/BP_PlayerCharacter.BP_PlayerCharacter_C|GetPlayerMesh (Variables|Default|GetPlayerPawn)) "ShootPoint" "0, 0, 0" "-40.000000, 0, 0")
      (bind (_isobjectmatch _hitactor) (Irrigation|ObjectDetection (Variables|Irrigation|GetDetectionRange)))
      (Variables|Irrigation|SetIrrigatedActor _hitactor)
      (if _isobjectmatch
        (Variables|Irrigation|SetIrrigatedActorRef (Variables|Irrigation|GetIrrigatedActor))
        (Class|BPIIrrigable|Irrigableon(Message) (Variables|Irrigation|GetIrrigatedActor))
        (else
          (Class|BPIIrrigable|IrrigableOff(Message) (Variables|Irrigation|GetIrrigatedActorRef))
          (Variables|Irrigation|SetIrrigatedActorRef 0))))
    (else
      (Variables|Irrigation|SetIrrigationSlow 1.0))))

(event Input|KeyboardEvents|AnyKey
  (params (Key :type Key%20Structure :default "None"))
  ;[0.9951 0.3077 1] Input Detection
  (:Pressed
    (Variables|Default|SetIsAnyKeyPressed true)
    (Variables|Default|SetIsGamepadInput (Class|KismetInputLibrary|KeyIsGamepadKey Key)))
  (:Released
    (Variables|Default|SetIsAnyKeyPressed false)))

(fn ConstructionScript)

(fn UpdatePlayerAim
  (if (Variables|Default|GetIsGamepadInput)
    (Aim|UpdateThumbstickAim)
    (else
      (Aim|UpdateMouseAim))))

(fn GetMouseVelocity
  (bind _returnvalue (Game|GetPlayerController 0))
  (bind (_deltax _deltay) (Class|PlayerController|GetInputMouseDelta _returnvalue))
  (return (/ (Math|Vector2D|MakeVector2D _deltax _deltay) (Utilities|Time|GetWorldDeltaSeconds))))

(fn GetMouseAimDirection
  (bind _mousevelocity (Aim|GetMouseVelocity))
  ;[1 0.019 0] Deprecated but useful
  (return (Math|Interpolation|RInterpTo (Pawn|GetControlRotation (Game|GetPlayerController 0) :!class /Script/Engine.Controller) (Math|Rotator|MakeRotator 0.0 0.0 (Class|KismetMathLibrary|DegAtan2 (.x _mousevelocity) (.y _mousevelocity))) (Utilities|Time|GetWorldDeltaSeconds) (* (Variables|Aim|GetMouseSmoothingStrength) (Variables|Irrigation|GetIrrigationSlow)))))

(fn IsMouseAboveDeadzone
  (return (> (Math|Vector2D|Vector2DLength (Aim|GetMouseVelocity)) (Variables|Aim|GetMouseDeadzone))))

(fn ObjectDetection
  (params (Range :type Float%20%28single-precision%29))
  (bind _playerpawn (Variables|Default|GetPlayerPawn))
  (bind _returnvalue (Transformation|GetActorLocation _playerpawn))
  (bind (_outhit _returnvalue_2) (Collision|SphereTraceForObjects _returnvalue (+ _returnvalue (* (Math|Vector|GetForwardVector (Pawn|GetControlRotation :!class /Script/Engine.Controller)) Range)) 5e+01 (Utilities|Array|MakeArray "ObjectTypeQuery1" "ObjectTypeQuery2") false (Utilities|Array|MakeArray self (Pawn|GetControlledPawn)) "None"))
  (return _returnvalue_2 (.HitActor (Collision|BreakHitResult _outhit))))

(fn CalculateDashDestination
  (return (+ (Transformation|GetActorLocation (Variables|Default|GetPlayerPawn)) (* (Math|Vector|GetForwardVector (Math|Rotator|MakeRotator 0.0 0.0 (Class|KismetMathLibrary|DegAtan2 (Input|AxisValues|GetMoveRight) (Input|AxisValues|GetMoveForward)))) (Variables|Dash|GetDashLength)))))

(fn UpdateMouseAim
  (bind (_pointfound _returnvalue) (Aim|GetMouseMappingtoRotation))
  (if _pointfound
    (Pawn|SetControlRotation _returnvalue)))

(fn GetThumbstickAimDirection
  (return (Math|Rotator|MakeRotator 0.0 0.0 (Class|KismetMathLibrary|DegAtan2 (Input|AxisValues|GetFireRight) (Input|AxisValues|GetFireForward)))))

(fn UpdateThumbstickAim
  (if (Aim|IsThumbstickAboveDeadzone)
    (Pawn|SetControlRotation (Game|GetPlayerController 0) (Aim|GetThumbstickAimDirection))))

(fn IsThumbstickAboveDeadzone
  (return (> (Math|Vector2D|Vector2DLength (Math|Vector2D|MakeVector2D (Input|AxisValues|GetFireForward) (Input|AxisValues|GetFireRight))) (Variables|Default|GetThumbstickDeadzone))))

(fn GetLineandPlaneIntersectionPoint
  (params (RayOrigin :type Vector) (RayDirection :type Vector) (Range :type Float%20%28single-precision%29) (PlaneOrigin :type Vector) (PlaneNormal :type Vector :default "0,0,1.000000"))
  (bind _returnvalue (* RayDirection Range))
  (bind _returnvalue_2 (+ RayOrigin _returnvalue))
  (bind _returnvalue_3 (- _returnvalue_2 RayOrigin))
  (bind _returnvalue_4 (Math|Vector|DotProduct _returnvalue_3 PlaneNormal))
  (return (+ (* _returnvalue_3 (/ (Math|Vector|DotProduct (- PlaneOrigin RayOrigin) PlaneNormal) _returnvalue_4)) RayOrigin) (!= _returnvalue_4 0.0)))

(fn GetMouseMappingtoRotation
  (bind (_worldlocation _worlddirection) (Game|Player|ConvertMouseLocationToWorldSpace))
  (bind _playerpawn (Variables|Default|GetPlayerPawn))
  (bind _returnvalue (Transformation|GetActorLocation _playerpawn))
  (bind _springarm (Variables|/Game/Blueprints/Player/BP_PlayerCharacter.BP_PlayerCharacter_C|GetSpringArm _playerpawn))
  (bind _targetarmlength (Variables|/Script/Engine.SpringArmComponent|GetTargetArmLength _springarm))
  (bind (_intersectionpoint _pointfound) (Aim|GetLineandPlaneIntersectionPoint _worldlocation _worlddirection _targetarmlength _returnvalue "0,0,1.000000"))
  (return _pointfound (Math|Rotator|FindLookatRotation _returnvalue _intersectionpoint)))

(fn SubtractWater
  (params (Continuous :type Boolean))
  (if Continuous
    (Default|ModifyWaterLevel (Variables|Default|GetPlayerPawn) (* (Variables|Default|GetSubtractedWaterAmount) -1.0 (Utilities|Time|GetWorldDeltaSeconds)))
    (else
      (Default|ModifyWaterLevel (Variables|Default|GetPlayerPawn) (* (Variables|Default|GetSubtractedWaterAmount) -1.0)))))