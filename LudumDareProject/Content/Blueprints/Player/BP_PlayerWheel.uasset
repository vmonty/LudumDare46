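; BP_PlayerWheel is the player character's wheel, which turns toward the direction of travel and emits movement dust.
; The construction script prints the parent actor's name and caches it as a BP_PlayerCharacter reference.
; Each Tick feeds player speed into the dust particles' Spawn parameter and, while moving, sets relative yaw from velocity direction minus player yaw.
; A node for setting dust direction from reversed velocity is left unconnected.
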(event EventBeginPlay)

(event Collision|EventActorBeginOverlap
  (params (OtherActor :type Actor%20Object%20Reference)))

(event EventTick
  (params (DeltaSeconds :type Float%20%28single-precision%29))
  (bind _returnvalue (Transformation|GetActorLocation))
  (bind _playerref (Variables|Default|GetPlayerRef))
  (bind _returnvalue_2 (Transformation|GetVelocity _playerref))
  (bind _returnvalue_3 (Math|Vector|VectorLength _returnvalue_2))
  (Utilities|IsValid _playerref
    (:Is%20Valid
      (Utilities|FlowControl|Sequence
        (:then_0
          ;[1 1 1] VFX parameters
          (Effects|Components|ParticleSystem|SetFloatParameter (Variables|Default|GetPS_PlayerMovementDust) "Spawn" _returnvalue_3))
        (:then_1
          ;[1 1 1] Update wheel rotation towards velocity
          (if (> _returnvalue_3 0.0)
            (Transformation|SetActorRelativeTransform (Math|Transform|MakeTransform "0, 0, 0" (Math|Rotator|MakeRotator 0.0 0.0 (- (.yaw (Math|Rotator|FindLookatRotation _returnvalue (+ _returnvalue_2 _returnvalue))) (.yaw (Transformation|GetActorRotation _playerref)))) "1,1,1") true false)))))))

(fn ConstructionScript
  (bind _returnvalue (Actor|GetParentActor))
  (Development|PrintString (Utilities|GetDisplayName _returnvalue))
  (bind _asbp_player_character (Utilities|Casting|CastToBP_PlayerCharacter _returnvalue))
  (Variables|Default|SetPlayerRef _asbp_player_character))