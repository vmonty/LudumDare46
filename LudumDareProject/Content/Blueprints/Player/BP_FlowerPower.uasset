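; BP_FlowerPower is a flower mesh actor, parented to BP_PlayerCharacter, meant to visualize the player's health through its materials.
; BeginPlay caches the parent's health component and puts two dynamic flower material instances on the mesh.
; Tick writes CalculateHealthValueForShader into both materials' "Life" parameter.
; That function contains an inverted, clamped normalization of current health, which appears unconnected to any output.
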(event EventBeginPlay
  (bind _sm_flowerpower (Variables|Default|GetSM_FlowerPower))
  (bind _asbp_player_character (Utilities|Casting|CastToBP_PlayerCharacter (Actor|GetParentActor)))
  (Variables|Default|SethealthComp (Variables|/Game/Blueprints/Player/BP_PlayerCharacter.BP_PlayerCharacter_C|GetBP_Health_Component _asbp_player_character))
  (bind _returnvalue (Rendering|Material|CreateDynamicMaterialInstance "/Game/Materials/Player/Water/M_Flower_Inst.M_Flower_Inst" "Flow01" :!class /Script/Engine.KismetMaterialLibrary))
  (bind _output_get (Variables|Default|SetM_Flow01 _returnvalue))
  (bind _returnvalue_2 (Rendering|Material|CreateDynamicMaterialInstance "/Game/Materials/Player/Water/M_Flower_Inst1.M_Flower_Inst1" "Flow02" :!class /Script/Engine.KismetMaterialLibrary))
  (bind _output_get_2 (Variables|Default|SetFlow02 _returnvalue_2))
  (Rendering|Material|SetMaterial _sm_flowerpower 0 _output_get)
  (Rendering|Material|SetMaterial _sm_flowerpower 1 _output_get_2))

(event EventTick
  (params (DeltaSeconds :type Float%20%28single-precision%29))
  (bind _returnvalue (|CalculateHealthValueForShader))
  (Utilities|IsValid (Variables|Default|GethealthComp)
    (:Is%20Valid
      (Rendering|Material|SetScalarParameterValue (Variables|Default|GetFlow02) "Life" _returnvalue :!class /Script/Engine.MaterialInstanceDynamic)
      (Rendering|Material|SetScalarParameterValue (Variables|Default|GetM_Flow01) "Life" _returnvalue :!class /Script/Engine.MaterialInstanceDynamic))))

(fn ConstructionScript)